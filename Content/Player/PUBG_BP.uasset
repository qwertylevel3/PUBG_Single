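; Player character Blueprint that handles third-person movement, mouse-look and sprinting.
; Move axes drive input along control-yaw directions, while Turn and LookUp rotate the controller.
; The Run action plays and reverses a timeline that ramps max walk speed.
; Tick switches rotation mode by velocity: the body follows controller yaw while moving and frees it when nearly stopped, so the face can be seen.
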(event `InputAxis|MoveForward`
  (params (AxisValue :type "Float (single-precision)"))
  ;[1 1 1] 基本平移
  (`self.AddMovementInput` (`KismetMathLibrary.GetForwardVector` (`KismetMathLibrary.MakeRotator` 0.0 0.0 (.yaw (`self.GetControlRotation`)))) AxisValue))

(event `InputAxis|MoveRight`
  (params (AxisValue :type "Float (single-precision)"))
  ;[1 1 1] 基本平移
  (`self.AddMovementInput` (`KismetMathLibrary.GetRightVector` (`KismetMathLibrary.MakeRotator` 0.0 0.0 (.yaw (`self.GetControlRotation`)))) AxisValue))

(event `InputAction|Run`
  (params (Key :type "Key Structure"))
  ;[1 1 1] shift 加速
  (:`Pressed`
    (bind (_direction _run) (`Timeline|RunTineLine` :!label _label)
      (:`Update`
        (set `CharacterMovementComponent.MaxWalkSpeed` _run (`self.CharacterMovement`)))))
  (:`Released`
    (goto _label :!via `Reverse`)))

(event `InputAxis|Turn`
  (params (AxisValue :type "Float (single-precision)"))
  ;[1 1 1] turn&& look up
  (`self.AddControllerYawInput` AxisValue))

(event `InputAxis|LookUp`
  (params (AxisValue :type "Float (single-precision)"))
  ;[1 1 1] turn&& look up
  (`self.AddControllerPitchInput` AxisValue))

(event `self.ReceiveTick`
  (params (DeltaSeconds :type "Float (single-precision)"))
  (bind _charactermovement (`self.CharacterMovement`))
  ;[1 1 1] 行走的时候看不到脸，停止的时候能看到脸
  (if (>= (`KismetMathLibrary.VSize` (`self.GetVelocity`)) 10.0)
    (set `CharacterMovementComponent.bOrientRotationToMovement` false _charactermovement)
    (set `self.bUseControllerRotationYaw` true)
    (else
      (set `CharacterMovementComponent.bOrientRotationToMovement` true _charactermovement)
      (set `self.bUseControllerRotationYaw` false))))

(fn `UserConstructionScript`)